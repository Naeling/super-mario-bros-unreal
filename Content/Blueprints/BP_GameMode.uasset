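; Game mode for a Mario-style game that tracks a countdown timer, coin count and lives.
; Tick counts the timer down and, once it runs out, prints a kill-Mario message every frame as a placeholder.
; IncrementCoins grants a life through IncrementLives when the count hits 100, without resetting coins.
; DecrementLives only prints a game-over message when lives drop below zero.
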(event EventBeginPlay)

(event EventTick
  (params (DeltaSeconds :type Float%20%28single-precision%29))
  (bind _output_get (Variables|Default|SetTimer (- (Variables|Default|GetTimer) DeltaSeconds)))
  (if (<= _output_get 0.0)
    (Development|PrintString "KILL MARIO")))

(fn ConstructionScript)

(fn IncrementCoins
  (bind _result (Math|Integer|IncrementInt (Variables|Default|GetCoins))
    (:%20%20
      (if (== _result 100)
        (CallFunction|IncrementLives)))))

(fn IncrementLives
  (Math|Integer|IncrementInt (Variables|Default|GetLives)))

(fn DecrementLives
  (bind _result (Math|Integer|DecrementInt (Variables|Default|GetLives))
    (:%20%20
      (if (< _result 0)
        (Development|PrintString "GAME OVER")))))