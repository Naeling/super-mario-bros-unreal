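; BP_FlagPole is a Mario-style flagpole prop that lowers its flag while the player character slides down it.
; Pole overlap on a custom collision channel snaps the flag down toward the actor's height, clamped, then starts BP_SpriteCharacter's pole slide.
; Tick then lowers the flag by a fixed per-frame offset, not delta-time scaled, until it passes a bottom limit and stops the slide.
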(event OnComponentBeginOverlap(PoleCollision)
  (params (OverlappedComponent :type Primitive%20Component%20Object%20Reference) (OtherActor :type Actor%20Object%20Reference) (OtherComp :type Primitive%20Component%20Object%20Reference) (OtherBodyIndex :type Integer) (bFromSweep :type Boolean) (SweepResult :type Hit%20Result%20Structure%20%28by%20ref%29))
  (if (Utilities|Enum|Equal(Enum) (Collision|GetCollisionObjectType OtherComp) "ECC_GameTraceChannel2")
    (Transformation|AddLocalOffset (Variables|Default|GetFlag) (Math|Vector|MakeVector 0.0 0.0 (Math|Float|Clamp(Float) (- (.z (Transformation|GetActorLocation OtherActor)) (.z (Transformation|GetWorldLocation (Variables|Default|GetFlag)))) -128.0 0.0)) false false)
    (Variables|Default|SetFlagIsGoingDown true)
    (bind _asbp_sprite_character (Utilities|Casting|CastToBP_SpriteCharacter OtherActor))
    (bind _output_get (Variables|Default|SetMario%20Actor _asbp_sprite_character))
    (Default|StartPoleSlide _output_get (Variables|Default|GetFlagLoweringSpeed))))

(event Custom|LowerFlag
  (Transformation|AddLocalOffset (Variables|Default|GetFlag) (Math|Vector|MakeVector 0.0 0.0 (Variables|Default|GetFlagLoweringSpeed)) false false)
  (if (< (.z (Variables|/Script/Engine.SceneComponent|GetRelativeLocation (Variables|Default|GetFlag))) -64.0)
    (Variables|Default|SetFlagIsGoingDown false)
    (Default|StopPoleSlide (Variables|Default|GetMario%20Actor))))

(event EventBeginPlay)

(event Collision|EventActorBeginOverlap
  (params (OtherActor :type Actor%20Object%20Reference)))

(event EventTick
  (params (DeltaSeconds :type Float%20%28single-precision%29))
  (if (Variables|Default|GetFlagIsGoingDown)
    (CallFunction|LowerFlag)))

(fn ConstructionScript)