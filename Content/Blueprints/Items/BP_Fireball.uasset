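; Bouncing fireball projectile, a Paper2D flipbook on a physics sphere that travels horizontally in a set direction and explodes on hitting a wall.
; BeginPlay builds up and down velocity vectors and launches it downward.
; Vertical hits send it upward until Tick sees it reach the bounce height above the impact point, then it inverts downward, producing a zigzag.
; Horizontal hits stop it, swap in the explosion flipbook and destroy it shortly after.
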(event OnComponentHit(Sphere)
  (params (HitComponent :type Primitive%20Component%20Object%20Reference) (OtherActor :type Actor%20Object%20Reference) (OtherComp :type Primitive%20Component%20Object%20Reference) (NormalImpulse :type Vector :default "0, 0, 0") (Hit :type Hit%20Result%20Structure%20%28by%20ref%29))
  (if (> (Math|Float|Absolute(Float) (.z NormalImpulse)) 0.0)
    (Physics|SetPhysicsLinearVelocity (Variables|Default|GetSphere) (Variables|Default|GetUpwardTrajectoryVector) false "None")
    (Variables|Default|SetCurrentBounceTargetHeight (+ (Variables|Default|GetBounceHeight) (.z (.location Hit))))
    (Variables|Default|SetIsMovingUpward true)
    (elif (> (Math|Float|Absolute(Float) (.x NormalImpulse)) 0.0)
      (CallFunction|Explode))))

(event Custom|Explode
  (Transformation|SetActorScale3D "0.500000,0.500000,0.500000")
  (Physics|SetPhysicsLinearVelocity (Variables|Default|GetSphere) "0, 0, 0" false "None")
  (Sprite|SetFlipbook (Variables|Default|GetPaperFlipbook) "/Game/Sprites/Items/FireFlower/FireBall/Explosion/FB_Fireball_Explosion.FB_Fireball_Explosion")
  (Utilities|Time|SetTimerbyEvent (delegate Custom|EndExplodeTimer) 0.1))

(event Custom|EndExplodeTimer
  (Actor|DestroyActor))

(event EventBeginPlay
  (CallFunction|InitializeTrajectoryVectors)
  (Physics|SetPhysicsLinearVelocity (Variables|Default|GetSphere) (Variables|Default|GetDownwardTrajectoryVector) false "None"))

(event Collision|EventActorBeginOverlap
  (params (OtherActor :type Actor%20Object%20Reference)))

(event EventTick
  (params (DeltaSeconds :type Float%20%28single-precision%29))
  (bind _mustinverttrajectory (CallFunction|MustInvertTrajectory))
  (if _mustinverttrajectory
    (Physics|SetPhysicsLinearVelocity (Variables|Default|GetSphere) (Variables|Default|GetDownwardTrajectoryVector) false "None")
    (Variables|Default|SetIsMovingUpward false)))

(fn ConstructionScript)

(fn InitializeTrajectoryVectors
  (Variables|Default|SetHorizontalSpeed (* (Variables|Default|GetHorizontalSpeed) (Variables|Default|GetHorizontalDirection)))
  (Variables|Default|SetUpwardTrajectoryVector (Math|Vector|MakeVector (Variables|Default|GetHorizontalSpeed) 0.0 (Variables|Default|GetVerticalSpeed)))
  (Variables|Default|SetDownwardTrajectoryVector (Math|Vector|MakeVector (Variables|Default|GetHorizontalSpeed) 0.0 (* (Variables|Default|GetVerticalSpeed) -1.0))))

(fn MustInvertTrajectory
  (return (and (Variables|Default|GetIsMovingUpward) (>= (.z (Transformation|GetActorLocation)) (Variables|Default|GetCurrentBounceTargetHeight)))))