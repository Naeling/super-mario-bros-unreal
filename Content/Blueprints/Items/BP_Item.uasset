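; BP_Item is a base Mario power-up item that emerges upward, walks sideways and is collected on touch.
; Spawn switches the capsule's collision channel and forces upward velocity each tick until an actor overlap ends, which restores another channel.
; While walking, it moves along X and reverses when X velocity is zero.
; Overlapping Mario, identified by class-name string, calls the empty TriggerMarioPowerup hook, then destroys the item.
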(event Custom|ApplySpawnVelocity
  (Variables|/Script/Engine.MovementComponent|SetVelocity (Variables|Character|GetCharacterMovement) (Math|Vector|MakeVector 0.0 0.0 (Variables|Default|GetSpawnVelocity))))

(event Custom|ManageWalkState
  (if (Pawn|Components|CharacterMovement|IsWalking (Variables|Character|GetCharacterMovement))
    (CallFunction|UpdateWalkVelocity)))

(event Custom|UpdateWalkVelocity
  (bind _isblocked (CallFunction|IsBlocked))
  (if _isblocked
    (CallFunction|InvertWalkDirection))
  (bind _walkvelocity (CallFunction|ComputeWalkVelocity))
  (Variables|/Script/Engine.MovementComponent|SetVelocity (Variables|Character|GetCharacterMovement) _walkvelocity))

(event Custom|ManageSpawnState
  (if (Variables|Default|GetIsSpawning)
    (CallFunction|ApplySpawnVelocity)))

(event Custom|Spawn
  (Collision|SetCollisionObjectType (Variables|Collision|GetCapsuleComponent) "ECC_GameTraceChannel1")
  (Variables|Default|SetIsSpawning true))

(event Custom|ManageMarioOverlap
  (params (MarioActor :type BP%20Sprite%20Character%20Object%20Reference))
  (CallFunction|TriggerMarioPowerup MarioActor)
  (Actor|DestroyActor))

(event EventTick
  (params (DeltaSeconds :type Float%20%28single-precision%29))
  (CallFunction|ManageWalkState)
  (CallFunction|ManageSpawnState))

(event Collision|EventActorBeginOverlap
  (params (OtherActor :type Actor%20Object%20Reference))
  (bind _ismarioactor (CallFunction|IsMarioActor OtherActor))
  (if _ismarioactor
    (bind _asbp_sprite_character (Utilities|Casting|CastToBP_SpriteCharacter OtherActor))
    (CallFunction|ManageMarioOverlap _asbp_sprite_character)))

(event Collision|EventActorEndOverlap
  (params (OtherActor :type Actor%20Object%20Reference))
  (Collision|SetCollisionObjectType (Variables|Collision|GetCapsuleComponent) "ECC_GameTraceChannel6")
  (Variables|Default|SetIsSpawning false))

(fn ConstructionScript)

(fn IsBlocked
  (return (== (.X (Math|Vector|BreakVector (Variables|/Script/Engine.MovementComponent|GetVelocity (Variables|Character|GetCharacterMovement)))) 0.0)))

(fn InvertWalkDirection
  (Variables|Default|SetCurrentWalkDirection (* (Variables|Default|GetCurrentWalkDirection) -1)))

(fn ComputeWalkVelocity
  (bind _charactermovement (Variables|Character|GetCharacterMovement))
  (bind _velocity (Variables|/Script/Engine.MovementComponent|GetVelocity _charactermovement))
  (bind (_x _y _z) (Math|Vector|BreakVector _velocity))
  (return (Math|Vector|MakeVector (* (Variables|Default|GetCurrentWalkDirection) (Variables|Default|GetWalkSpeed)) _y _z)))

(fn IsMarioActor
  (params (Actor :type Actor%20Object%20Reference))
  (return (Utilities|Enum|Equal(Enum) (Utilities|GetClassDisplayName (Utilities|GetClass Actor)) "BP_SpriteCharacter_C")))

(fn TriggerMarioPowerup
  (params (Mario%20Actor :type BP%20Sprite%20Character%20Object%20Reference)))