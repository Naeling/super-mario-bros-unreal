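; BP_Jumping_Coin is a Mario-style coin pickup that animates vertically as soon as it spawns, with no overlap needed.
; A timeline started on BeginPlay drives the flipbook's relative Z, then destroys the actor and increments the coin count on BP_GameMode.
; Helper functions identify Mario by class-name string and test whether his capsule is below the coin, but nothing in this file calls them.
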(event EventBeginPlay
  (bind _flipbook (Variables|Default|GetFlipbook))
  (bind _relativelocation (Variables|/Script/Engine.SceneComponent|GetRelativeLocation _flipbook))
  (bind _updown (Timeline|Timeline PlayFromStart)
    (:Update
      (Transformation|SetRelativeLocation (Variables|Default|GetFlipbook) (Math|Vector|MakeVector (.x _relativelocation) (.y _relativelocation) _updown) false false))
    (:Finished
      (Actor|DestroyActor)
      (bind _asbp_game_mode (Utilities|Casting|CastToBP_GameMode (Game|GetGameMode)))
      (Default|IncrementCoins _asbp_game_mode))))

(event Collision|EventActorBeginOverlap
  (params (OtherActor :type Actor%20Object%20Reference)))

(event EventTick
  (params (DeltaSeconds :type Float%20%28single-precision%29)))

(fn ConstructionScript)

(fn IsMarioActor
  (params (Actor :type Actor%20Object%20Reference))
  (return (Utilities|Enum|Equal(Enum) (Utilities|GetClassDisplayName (Utilities|GetClass Actor)) "BP_SpriteCharacter_C")))

(fn IsMarioBelowSelf
  (params (Actor :type Actor%20Object%20Reference))
  (bind _returnvalue (Actor|GetComponentbyClass Actor "/Script/Engine.CapsuleComponent"))
  (bind (_origin _boxextent) (Collision|GetComponentBounds _returnvalue))
  (return (< (.Z (Math|Vector|BreakVector _origin)) (- (.Z (Math|Vector|BreakVector (Transformation|GetActorLocation))) (/ (.Z (Math|Vector|BreakVector _boxextent)) 4.0)))))