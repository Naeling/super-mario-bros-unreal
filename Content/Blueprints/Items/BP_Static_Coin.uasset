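; BP_Static_Coin is a coin item actor that destroys itself when any actor begins overlapping it.
; It awards nothing and does not filter the overlapping actor.
; Two helper functions go uncalled in the shown graphs: one identifies Mario by comparing the class display name to BP_SpriteCharacter_C.
; The other tests whether an actor's capsule center sits below the coin by over a quarter of its Z extent.
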(event Collision|EventActorBeginOverlap
  (params (OtherActor :type Actor%20Object%20Reference))
  (Actor|DestroyActor))

(event EventTick
  (params (DeltaSeconds :type Float%20%28single-precision%29)))

(fn ConstructionScript)

(fn IsMarioActor
  (params (Actor :type Actor%20Object%20Reference))
  (return (Utilities|Enum|Equal(Enum) (Utilities|GetClassDisplayName (Utilities|GetClass Actor)) "BP_SpriteCharacter_C")))

(fn IsMarioBelowSelf
  (params (Actor :type Actor%20Object%20Reference))
  (bind _returnvalue (Actor|GetComponentbyClass Actor "/Script/Engine.CapsuleComponent"))
  (bind (_origin _boxextent) (Collision|GetComponentBounds _returnvalue))
  (return (< (.Z (Math|Vector|BreakVector _origin)) (- (.Z (Math|Vector|BreakVector (Transformation|GetActorLocation))) (/ (.Z (Math|Vector|BreakVector _boxextent)) 4.0)))))