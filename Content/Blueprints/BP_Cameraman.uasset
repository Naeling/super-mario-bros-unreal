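; Cameraman character that side-scrolls along +X after Mario, never following backward.
; On BeginPlay it finds the Mario actor, and the ForwardMoveDetection overlap toggles forward movement, zeroing velocity when Mario leaves.
; While active, Tick sets CharacterMovement velocity from Mario's positive X speed, scaled by their X offset so the follow eases toward full speed as Mario catches up.
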(event OnComponentBeginOverlap(ForwardMoveDetection)
  (params (OverlappedComponent :type Primitive%20Component%20Object%20Reference) (OtherActor :type Actor%20Object%20Reference) (OtherComp :type Primitive%20Component%20Object%20Reference) (OtherBodyIndex :type Integer) (bFromSweep :type Boolean) (SweepResult :type Hit%20Result%20Structure%20%28by%20ref%29))
  (if (== OtherActor (Variables|Default|GetMarioActor))
    (Variables|Default|SetIsMovingForward true)))

(event OnComponentEndOverlap(ForwardMoveDetection)
  (params (OverlappedComponent :type Primitive%20Component%20Object%20Reference) (OtherActor :type Actor%20Object%20Reference) (OtherComp :type Primitive%20Component%20Object%20Reference) (OtherBodyIndex :type Integer))
  (if (== OtherActor (Variables|Default|GetMarioActor))
    (Variables|Default|SetIsMovingForward false)
    (Variables|/Script/Engine.MovementComponent|SetVelocity (Variables|Character|GetCharacterMovement) (Math|Vector|MakeVector 0.0 0.0 0.0))))

(event EventBeginPlay
  (bind _returnvalue (Actor|GetActorOfClass (Variables|Default|GetMarioClass)))
  (Variables|Default|SetMarioActor _returnvalue))

(event EventTick
  (params (DeltaSeconds :type Float%20%28single-precision%29))
  (if (Variables|Default|GetIsMovingForward)
    (Variables|/Script/Engine.MovementComponent|SetVelocity (Variables|Character|GetCharacterMovement) (Math|Vector|MakeVector (* (Math|Float|Max(Float) (.x (Transformation|GetVelocity (Variables|Default|GetMarioActor))) 0.0) (+ (* (Math|Float|Min(Float) (/ (- 42.0 (- (.x (Transformation|GetActorLocation)) (.x (Transformation|GetActorLocation (Variables|Default|GetMarioActor))))) 42.0) 1.0) 0.9) 0.1)) 0.0 0.0))))

(fn ConstructionScript)