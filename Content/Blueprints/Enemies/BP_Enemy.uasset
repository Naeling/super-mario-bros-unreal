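; Base enemy character for a Mario-style game that detects contact with the player and distinguishes stomps from side hits.
; Capsule overlaps identify Mario by class name, then compare capsule bounds within a narrow height window to call empty jump-over or side-overlap functions.
; Tick caps fall speed.
; A death event freezes the sprite, disables capsule collision, rotates the actor and launches it in the given direction.
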(event OnComponentBeginOverlap(CapsuleComponent)
  (params (OverlappedComponent :type Primitive%20Component%20Object%20Reference) (OtherActor :type Actor%20Object%20Reference) (OtherComp :type Primitive%20Component%20Object%20Reference) (OtherBodyIndex :type Integer) (bFromSweep :type Boolean) (SweepResult :type Hit%20Result%20Structure%20%28by%20ref%29))
  (bind _ismarioactor (CallFunction|IsMarioActor OtherActor))
  (if _ismarioactor
    (CallFunction|ManageMarioOverlap OtherActor)))

(event Custom|StartDeathAnimation
  (params (Direction :type Float%20%28double-precision%29))
  (Character|Jump)
  (Components|Timeline|SetPlayRate (Variables|Default|GetSprite) 0.0)
  (Collision|SetCollisionEnabled (Variables|Collision|GetCapsuleComponent) "NoCollision")
  (Transformation|SetActorRotation "180.000000,0.000000,0.000000")
  (Variables|/Script/Engine.MovementComponent|SetVelocity (Variables|Character|GetCharacterMovement) (Math|Vector|MakeVector (* (Variables|Default|GetDeathAnimationHorizontalSpeed) Direction) 0.0 (Variables|Default|GetDeathAnimationVerticalSpeed))))

(event Custom|ApplyFallSpeedLimit
  (bind _charactermovement (Variables|Character|GetCharacterMovement))
  (if (< (.z (Variables|/Script/Engine.MovementComponent|GetVelocity (Variables|Character|GetCharacterMovement))) (Variables|Default|GetFallSpeedLimit))
    (Variables|/Script/Engine.MovementComponent|SetVelocity _charactermovement (Math|Vector|MakeVector (.x (Variables|/Script/Engine.MovementComponent|GetVelocity _charactermovement)) (.y (Variables|/Script/Engine.MovementComponent|GetVelocity _charactermovement)) (Variables|Default|GetFallSpeedLimit)))))

(event Custom|ManageMarioOverlap
  (params (MarioActor :type Actor%20Object%20Reference))
  (bind _ismarioaboveself (CallFunction|IsMarioAboveSelf MarioActor))
  (if _ismarioaboveself
    (bind _asbp_sprite_character (Utilities|Casting|CastToBP_SpriteCharacter MarioActor))
    (CallFunction|OnMarioJumpOver _asbp_sprite_character)
    (else
      (bind _asbp_sprite_character_2 (Utilities|Casting|CastToBP_SpriteCharacter MarioActor))
      (CallFunction|OnMarioSideOverlap _asbp_sprite_character_2))))

(event EventTick
  (params (DeltaSeconds :type Float%20%28single-precision%29))
  (CallFunction|ApplyFallSpeedLimit))

(event Collision|EventActorEndOverlap
  (params (OtherActor :type Actor%20Object%20Reference))
  (bind _ismarioactor (CallFunction|IsMarioActor OtherActor))
  (if _ismarioactor
    _))

(fn ConstructionScript)

(fn IsMarioActor
  (params (Actor :type Actor%20Object%20Reference))
  (return (Utilities|Enum|Equal(Enum) (Utilities|GetClassDisplayName (Utilities|GetClass Actor)) "BP_SpriteCharacter_C")))

(fn IsMarioAboveSelf
  (params (Actor :type Actor%20Object%20Reference))
  (bind _upperbound (CallFunction|GetUpperComponentBound self))
  (bind _lowerbound (CallFunction|GetLowerComponentBound Actor))
  (if (and (< (- _upperbound _lowerbound) 4.0) (> (- _upperbound _lowerbound) 0.0))
    (return true)
    (else
      (return false))))

(fn OnMarioJumpOver
  (params (Mario :type BP%20Sprite%20Character%20Object%20Reference)))

(fn OnMarioSideOverlap
  (params (Mario :type BP%20Sprite%20Character%20Object%20Reference)))

(fn GetUpperComponentBound
  (params (Actor :type Actor%20Object%20Reference))
  (bind _returnvalue (Actor|GetComponentbyClass Actor "/Script/Engine.CapsuleComponent"))
  (bind (_origin _boxextent) (Collision|GetComponentBounds _returnvalue))
  (return (+ (.Z (Math|Vector|BreakVector _origin)) (.Z (Math|Vector|BreakVector _boxextent)))))

(fn GetLowerComponentBound
  (params (Actor :type Actor%20Object%20Reference))
  (bind _returnvalue (Actor|GetComponentbyClass Actor "/Script/Engine.CapsuleComponent"))
  (bind (_origin _boxextent) (Collision|GetComponentBounds _returnvalue))
  (return (- (.Z (Math|Vector|BreakVector _origin)) (.Z (Math|Vector|BreakVector _boxextent)))))

(fn IsFireballActor
  (params (Actor :type Actor%20Object%20Reference)))