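; Enemy for a Mario-style platformer that patrols along X and dies when Mario jumps on it.
; Each tick while walking it drives CharacterMovement velocity directly, reversing direction when X velocity is zero, and holds still once dead.
; Parent-class overlap hooks decide the outcome: side contact kills Mario unless the enemy is dead.
; A stomp bounces Mario upward, marks it dead and destroys it immediately or after a death delay.
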(event Custom|EndDeathTimerEvent
  (Actor|DestroyActor))

(event Custom|ManageWalkState
  (if (Pawn|Components|CharacterMovement|IsWalking (Variables|Character|GetCharacterMovement))
    (CallFunction|UpdateWalkVelocity)))

(event Custom|UpdateWalkVelocity
  (if (Variables|Default|GetIsDead)
    (Variables|/Script/Engine.MovementComponent|SetVelocity (Variables|Character|GetCharacterMovement) "0, 0, 0")
    (else
      (bind _isblocked (CallFunction|IsBlocked))
      (if _isblocked
        (CallFunction|InvertWalkDirection))
      (bind _walkvelocity (CallFunction|ComputeWalkVelocity))
      (Variables|/Script/Engine.MovementComponent|SetVelocity (Variables|Character|GetCharacterMovement) _walkvelocity))))

(event EventTick
  (params (DeltaSeconds :type Float%20%28single-precision%29))
  (|CallParentFunction 0.0)
  (CallFunction|ManageWalkState))

(event Collision|EventActorBeginOverlap
  (params (OtherActor :type Actor%20Object%20Reference))
  (|CallParentFunction OtherActor) ; This node is disabled and will not be called.\nDrag off pins to build functionality.
)

(fn ConstructionScript
  (|CallParentFunction))

(fn OnMarioJumpOver
  (params (Mario :type BP%20Sprite%20Character%20Object%20Reference))
  (bind _deathdelay (Variables|Default|GetDeathDelay))
  (|CallParentFunction Mario)
  (if (> _deathdelay 0.0)
    (Utilities|Time|SetTimerbyEvent (EventDispatchers|CreateEvent :!event Custom|EndDeathTimerEvent) _deathdelay)
    (else
      (CallFunction|EndDeathTimerEvent)))
  (if (not (Variables|Default|GetIsDead))
    (CallFunction|MakeMarioJump Mario)
    (Variables|Default|SetIsDead true)))

(fn MakeMarioJump
  (params (Mario :type BP%20Sprite%20Character%20Object%20Reference))
  (bind _returnvalue (Actor|GetComponentbyClass Mario "/Script/Engine.CharacterMovementComponent"))
  (Variables|/Script/Engine.MovementComponent|SetVelocity _returnvalue (Math|Vector|MakeVector (.X (Math|Vector|BreakVector (Variables|/Script/Engine.MovementComponent|GetVelocity _returnvalue))) (.Y (Math|Vector|BreakVector (Variables|/Script/Engine.MovementComponent|GetVelocity _returnvalue))) (Variables|Default|GetMarioKillJumpVelocity))))

(fn OnMarioSideOverlap
  (params (Mario :type BP%20Sprite%20Character%20Object%20Reference))
  (|CallParentFunction Mario)
  (if (not (Variables|Default|GetIsDead))
    (Default|EnemyKillMario Mario)))

(fn IsBlocked
  (return (== (.X (Math|Vector|BreakVector (Variables|/Script/Engine.MovementComponent|GetVelocity (Variables|Character|GetCharacterMovement)))) 0.0)))

(fn InvertWalkDirection
  (Variables|Default|SetCurrentWalkDirection (* (Variables|Default|GetCurrentWalkDirection) -1)))

(fn ComputeWalkVelocity
  (bind _charactermovement (Variables|Character|GetCharacterMovement))
  (bind _velocity (Variables|/Script/Engine.MovementComponent|GetVelocity _charactermovement))
  (bind (_x _y _z) (Math|Vector|BreakVector _velocity))
  (return (Math|Vector|MakeVector (* (Variables|Default|GetCurrentWalkDirection) (Variables|Default|GetWalkSpeed)) _y _z)))