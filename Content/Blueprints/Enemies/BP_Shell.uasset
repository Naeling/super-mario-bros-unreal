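; BP_Shell is a Mario-style shell enemy that can be kicked along X and kills Mario on side contact while moving.
; Tick overrides X velocity while walking, and wall hits reverse direction.
; Side-touching an idle shell launches it away from Mario; stomping a moving one stops it and bounces Mario, while stomping an idle one sets zero direction.
; Starting ignores Mario collision until a reversal or stop restores overlap.
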(event OnComponentHit(CapsuleComponent)
  (params (HitComponent :type Primitive%20Component%20Object%20Reference) (OtherActor :type Actor%20Object%20Reference) (OtherComp :type Primitive%20Component%20Object%20Reference) (NormalImpulse :type Vector :default "0, 0, 0") (Hit :type Hit%20Result%20Structure%20%28by%20ref%29))
  (if (> (Math|Float|Absolute(Float) (.x (.normal Hit))) 0.0)
    (CallFunction|InvertWalkDirection)))

(event Custom|ManageWalkState
  (if (Pawn|Components|CharacterMovement|IsWalking (Variables|Character|GetCharacterMovement))
    (CallFunction|UpdateWalkVelocity)))

(event Custom|UpdateWalkVelocity
  (bind _charactermovement (Variables|Character|GetCharacterMovement))
  (if (Variables|Default|GetIsMoving)
    (bind _walkvelocity (CallFunction|ComputeWalkVelocity))
    (Variables|/Script/Engine.MovementComponent|SetVelocity (Variables|Character|GetCharacterMovement) _walkvelocity)
    (else
      (Variables|/Script/Engine.MovementComponent|SetVelocity _charactermovement (Math|Vector|MakeVector 0.0 (.y (Variables|/Script/Engine.MovementComponent|GetVelocity _charactermovement)) (.z (Variables|/Script/Engine.MovementComponent|GetVelocity _charactermovement)))))))

(event EventTick
  (params (DeltaSeconds :type Float%20%28single-precision%29))
  (CallFunction|ManageWalkState))

(event Collision|EventActorBeginOverlap
  (params (OtherActor :type Actor%20Object%20Reference))
  (|CallParentFunction OtherActor) ; This node is disabled and will not be called.\nDrag off pins to build functionality.
)

(event EventBeginPlay)

(fn ConstructionScript
  (|CallParentFunction))

(fn IsBlocked
  (return (== (.X (Math|Vector|BreakVector (Variables|/Script/Engine.MovementComponent|GetVelocity (Variables|Character|GetCharacterMovement)))) 0.0)))

(fn InvertWalkDirection
  (Variables|Default|SetCurrentWalkDirection (* (Variables|Default|GetCurrentWalkDirection) -1))
  (CallFunction|ActivateCollisionwithMario))

(fn ComputeWalkVelocity
  (bind _charactermovement (Variables|Character|GetCharacterMovement))
  (bind _velocity (Variables|/Script/Engine.MovementComponent|GetVelocity _charactermovement))
  (bind (_x _y _z) (Math|Vector|BreakVector _velocity))
  (return (Math|Vector|MakeVector (* (Variables|Default|GetCurrentWalkDirection) (Variables|Default|GetWalkSpeed)) _y _z)))

(fn OnMarioSideOverlap
  (params (Mario :type BP%20Sprite%20Character%20Object%20Reference))
  (|CallParentFunction Mario)
  (if (Variables|Default|GetIsMoving)
    (Default|EnemyKillMario Mario)
    (else
      (Variables|Default|SetIsMoving true)
      (bind _movedirection (CallFunction|ComputeMoveDirection Mario))
      (CallFunction|StartMoving _movedirection true))))

(fn OnMarioJumpOver
  (params (Mario :type BP%20Sprite%20Character%20Object%20Reference))
  (|CallParentFunction Mario)
  (if (Variables|Default|GetIsMoving)
    (CallFunction|MakeMarioJump Mario)
    (CallFunction|StopMoving)
    (else
      (CallFunction|StartMoving 0.0 true))))

(fn MakeMarioJump
  (params (MarioActor :type Actor%20Object%20Reference))
  (bind _returnvalue (Actor|GetComponentbyClass MarioActor "/Script/Engine.CharacterMovementComponent"))
  (Variables|/Script/Engine.MovementComponent|SetVelocity _returnvalue (Math|Vector|MakeVector (.X (Math|Vector|BreakVector (Variables|/Script/Engine.MovementComponent|GetVelocity _returnvalue))) (.Y (Math|Vector|BreakVector (Variables|/Script/Engine.MovementComponent|GetVelocity _returnvalue))) (Variables|Default|GetMarioKillJumpVelocity))))

(fn StartMoving
  (params (MoveDirection :type Float%20%28double-precision%29) (DisableCollisionWithMario :type Boolean))
  (Variables|Default|SetCurrentWalkDirection MoveDirection)
  (Variables|Default|SetIsMoving true)
  (if DisableCollisionWithMario
    (Collision|SetCollisionResponsetoChannel (Variables|Default|GetCapsuleComponent) "ECC_GameTraceChannel2" "ECR_Ignore")))

(fn ActivateCollisionwithMario
  (Collision|SetCollisionResponsetoChannel (Variables|Default|GetCapsuleComponent) "ECC_GameTraceChannel2" "ECR_Overlap"))

(fn StopMoving
  (CallFunction|ActivateCollisionwithMario)
  (Variables|Default|SetIsMoving false))

(fn ComputeMoveDirection
  (params (Mario%20Actor :type BP%20Sprite%20Character%20Object%20Reference))
  (if (>= (- (.x (Transformation|GetActorLocation)) (.x (Transformation|GetActorLocation Mario%20Actor))) 0.0)
    (return 1.0)
    (else
      (return -1.0))))