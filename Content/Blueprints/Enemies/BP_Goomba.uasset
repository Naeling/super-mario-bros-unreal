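; BP_Goomba is a Goomba enemy Blueprint for a Mario-style game, built on a parent class that supplies its base behavior.
; Its only custom logic overrides On Mario Jump Over, calling the parent, switching the sprite to the death flipbook and shrinking the capsule to a tiny size.
; Tick and construction only forward to the parent, while BeginPlay and overlap events are disabled placeholders.
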(event EventBeginPlay
  (|CallParentFunction) ; This node is disabled and will not be called.\nDrag off pins to build functionality.
)

(event Collision|EventActorBeginOverlap
  (params (OtherActor :type Actor%20Object%20Reference))
  (|CallParentFunction OtherActor) ; This node is disabled and will not be called.\nDrag off pins to build functionality.
)

(event EventTick
  (params (DeltaSeconds :type Float%20%28single-precision%29))
  (|CallParentFunction DeltaSeconds))

(fn ConstructionScript
  (|CallParentFunction))

(fn OnMarioJumpOver
  (params (Mario :type BP%20Sprite%20Character%20Object%20Reference))
  (|CallParentFunction Mario)
  (Sprite|SetFlipbook (Variables|Default|GetSprite) "/Game/Sprites/Enemies/Goomba/Die/FB_Goomba_Die.FB_Goomba_Die")
  (Components|Capsule|SetCapsuleSize (Variables|Default|GetCapsuleComponent) 2.0 2.0 true))