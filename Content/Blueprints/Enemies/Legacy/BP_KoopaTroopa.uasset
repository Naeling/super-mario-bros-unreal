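; Koopa Troopa enemy that walks along X, can be stomped into a shell, and kills Mario on other contact.
; While walking, Tick sets horizontal velocity from direction and speed, reversing whenever X velocity reads zero (treated as blocked).
; Overlaps identify Mario by class display name, then compare heights using his capsule bounds.
; A stomp destroys the Koopa, spawns BP_Shell and bounces Mario; otherwise it calls EnemyKillMario.
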(event Custom|ManageWalkState
  (if (Pawn|Components|CharacterMovement|IsWalking (Variables|Character|GetCharacterMovement))
    (CallFunction|UpdateWalkVelocity)))

(event Custom|UpdateWalkVelocity
  (bind _isblocked (CallFunction|IsBlocked))
  (if _isblocked
    (CallFunction|InvertWalkDirection))
  (bind _horizontalvelocity (CallFunction|ComputeHorizontalVelocity (Variables|Default|GetWalkSpeed)))
  (Variables|/Script/Engine.MovementComponent|SetVelocity (Variables|Character|GetCharacterMovement) _horizontalvelocity))

(event Custom|ManageMarioOverlap
  (params (MarioActor :type Actor%20Object%20Reference))
  (bind _ismarioaboveself (CallFunction|IsMarioAboveSelf MarioActor))
  (if _ismarioaboveself
    (Development|PrintString "GOOMBA DIES")
    (Actor|DestroyActor)
    (Game|SpawnActorfromClass "/Game/Blueprints/Enemies/Legacy/BP_Shell.BP_Shell_C" (Transformation|GetActorTransform) "AlwaysSpawn" 0 0)
    (CallFunction|MakeMarioJump MarioActor)
    (else
      (Development|PrintString "MARIO DIES")
      (bind _asbp_sprite_character (Utilities|Casting|CastToBP_SpriteCharacter MarioActor)
        (:then
          (Default|EnemyKillMario _asbp_sprite_character)
          (Development|PrintString "CALLED KILL MARIO"))
        (:CastFailed
          (Development|PrintString "FAILED TO CAST"))))))

(event EventTick
  (params (DeltaSeconds :type Float%20%28single-precision%29))
  (CallFunction|ManageWalkState))

(event Collision|EventActorBeginOverlap
  (params (OtherActor :type Actor%20Object%20Reference))
  (bind _ismarioactor (CallFunction|IsMarioActor OtherActor))
  (if _ismarioactor
    (CallFunction|ManageMarioOverlap OtherActor)))

(fn ConstructionScript)

(fn IsBlocked
  (return (== (.X (Math|Vector|BreakVector (Variables|/Script/Engine.MovementComponent|GetVelocity (Variables|Character|GetCharacterMovement)))) 0.0)))

(fn InvertWalkDirection
  (Variables|Default|SetCurrentWalkDirection (* (Variables|Default|GetCurrentWalkDirection) -1)))

(fn ComputeHorizontalVelocity
  (params (BaseHorizontalVelocity :type Float%20%28double-precision%29))
  (bind _charactermovement (Variables|Character|GetCharacterMovement))
  (bind _velocity (Variables|/Script/Engine.MovementComponent|GetVelocity _charactermovement))
  (bind (_x _y _z) (Math|Vector|BreakVector _velocity))
  (return (Math|Vector|MakeVector (* (Variables|Default|GetCurrentWalkDirection) (Variables|Default|GetWalkSpeed)) _y _z)))

(fn IsMarioActor
  (params (Actor :type Actor%20Object%20Reference))
  (return (Utilities|Enum|Equal(Enum) (Utilities|GetClassDisplayName (Utilities|GetClass Actor)) "BP_SpriteCharacter_C")))

(fn IsMarioAboveSelf
  (params (Actor :type Actor%20Object%20Reference))
  (bind _returnvalue (Actor|GetComponentbyClass Actor "/Script/Engine.CapsuleComponent"))
  (bind (_origin _boxextent) (Collision|GetComponentBounds _returnvalue))
  (return (> (.Z (Math|Vector|BreakVector _origin)) (+ (/ (.Z (Math|Vector|BreakVector _boxextent)) 4.0) (.Z (Math|Vector|BreakVector (Transformation|GetActorLocation)))))))

(fn MakeMarioJump
  (params (MarioActor :type Actor%20Object%20Reference))
  (bind _returnvalue (Actor|GetComponentbyClass MarioActor "/Script/Engine.CharacterMovementComponent"))
  (Variables|/Script/Engine.MovementComponent|SetVelocity _returnvalue (Math|Vector|MakeVector (.X (Math|Vector|BreakVector (Variables|/Script/Engine.MovementComponent|GetVelocity _returnvalue))) (.Y (Math|Vector|BreakVector (Variables|/Script/Engine.MovementComponent|GetVelocity _returnvalue))) (Variables|Default|GetMarioKillJumpVelocity))))