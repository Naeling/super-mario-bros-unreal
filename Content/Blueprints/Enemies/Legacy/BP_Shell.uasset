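; BP_Shell is a Koopa-style shell enemy in a Mario platformer that Mario stomps to start or stop sliding.
; Tick sets horizontal velocity while walking, reversing direction whenever X velocity is zero, which also happens on starting from rest.
; Overlaps identify Mario by class name string and compare capsule height.
; A stomp toggles movement and bounces Mario, while other contact with a moving shell calls EnemyKillMario.
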(event Custom|ManageWalkState
  (if (Pawn|Components|CharacterMovement|IsWalking (Variables|Character|GetCharacterMovement))
    (CallFunction|UpdateWalkVelocity)))

(event Custom|UpdateWalkVelocity
  (bind _charactermovement (Variables|Character|GetCharacterMovement))
  (if (Variables|Default|GetIsMoving)
    (bind _isblocked (CallFunction|IsBlocked))
    (if _isblocked
      (CallFunction|InvertWalkDirection))
    (bind _walkvelocity (CallFunction|ComputeWalkVelocity))
    (Variables|/Script/Engine.MovementComponent|SetVelocity (Variables|Character|GetCharacterMovement) _walkvelocity)
    (else
      (Variables|/Script/Engine.MovementComponent|SetVelocity _charactermovement (Math|Vector|MakeVector 0.0 (.y (Variables|/Script/Engine.MovementComponent|GetVelocity _charactermovement)) (.z (Variables|/Script/Engine.MovementComponent|GetVelocity _charactermovement)))))))

(event Custom|ManageMarioOverlap
  (params (MarioActor :type Actor%20Object%20Reference))
  (bind _ismarioaboveself (CallFunction|IsMarioAboveSelf MarioActor))
  (if _ismarioaboveself
    (Development|PrintString "GOOMBA DIES")
    (Variables|Default|SetIsMoving (not (Variables|Default|GetIsMoving)))
    (CallFunction|MakeMarioJump MarioActor)
    (elif (Variables|Default|GetIsMoving)
      (Development|PrintString "MARIO DIES")
      (bind _asbp_sprite_character (Utilities|Casting|CastToBP_SpriteCharacter MarioActor)
        (:then
          (Default|EnemyKillMario _asbp_sprite_character)
          (Development|PrintString "CALLED KILL MARIO"))
        (:CastFailed
          (Development|PrintString "FAILED TO CAST"))))))

(event EventTick
  (params (DeltaSeconds :type Float%20%28single-precision%29))
  (CallFunction|ManageWalkState))

(event Collision|EventActorBeginOverlap
  (params (OtherActor :type Actor%20Object%20Reference))
  (bind _ismarioactor (CallFunction|IsMarioActor OtherActor))
  (if _ismarioactor
    (CallFunction|ManageMarioOverlap OtherActor)))

(fn ConstructionScript)

(fn IsBlocked
  (return (== (.X (Math|Vector|BreakVector (Variables|/Script/Engine.MovementComponent|GetVelocity (Variables|Character|GetCharacterMovement)))) 0.0)))

(fn InvertWalkDirection
  (Variables|Default|SetCurrentWalkDirection (* (Variables|Default|GetCurrentWalkDirection) -1)))

(fn ComputeWalkVelocity
  (bind _charactermovement (Variables|Character|GetCharacterMovement))
  (bind _velocity (Variables|/Script/Engine.MovementComponent|GetVelocity _charactermovement))
  (bind (_x _y _z) (Math|Vector|BreakVector _velocity))
  (return (Math|Vector|MakeVector (* (Variables|Default|GetCurrentWalkDirection) (Variables|Default|GetWalkSpeed)) _y _z)))

(fn IsMarioActor
  (params (Actor :type Actor%20Object%20Reference))
  (return (Utilities|Enum|Equal(Enum) (Utilities|GetClassDisplayName (Utilities|GetClass Actor)) "BP_SpriteCharacter_C")))

(fn IsMarioAboveSelf
  (params (Actor :type Actor%20Object%20Reference))
  (bind _returnvalue (Actor|GetComponentbyClass Actor "/Script/Engine.CapsuleComponent"))
  (bind (_origin _boxextent) (Collision|GetComponentBounds _returnvalue))
  (return (> (.Z (Math|Vector|BreakVector _origin)) (+ (/ (.Z (Math|Vector|BreakVector _boxextent)) 4.0) (.Z (Math|Vector|BreakVector (Transformation|GetActorLocation)))))))

(fn MakeMarioJump
  (params (MarioActor :type Actor%20Object%20Reference))
  (bind _returnvalue (Actor|GetComponentbyClass MarioActor "/Script/Engine.CharacterMovementComponent"))
  (Variables|/Script/Engine.MovementComponent|SetVelocity _returnvalue (Math|Vector|MakeVector (.X (Math|Vector|BreakVector (Variables|/Script/Engine.MovementComponent|GetVelocity _returnvalue))) (.Y (Math|Vector|BreakVector (Variables|/Script/Engine.MovementComponent|GetVelocity _returnvalue))) (Variables|Default|GetMarioKillJumpVelocity))))