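; CharacterSpawner is a component that makes an existing character emerge vertically from its owner's location.
; SpawnCharacter teleports the character there, disables input and switches its capsule to a custom collision channel, saving the original.
; Tick overrides movement velocity with a vertical speed while spawning.
; The capsule's first end-overlap event stops the forced movement and restores collision and input.
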(event Custom|EndSpawn
  (Variables|Default|SetIsSpawning false)
  (Collision|SetCollisionObjectType (Variables|/Script/Engine.Character|GetCapsuleComponent (Variables|Default|GetCharacterToSpawn)) (Variables|Default|GetInitialCollisionChannel))
  (Input|EnableInput (Variables|Default|GetCharacterToSpawn) 0))

(event Custom|SpawnCharacter
  (params (CharacterToSpawn :type Character%20Object%20Reference))
  (bind _output_get (Variables|Default|SetCharacterToSpawn CharacterToSpawn))
  (Transformation|SetActorLocation _output_get (Transformation|GetActorLocation (Components|GetOwner)) false false)
  (Variables|Default|SetInitialCollisionChannel (Collision|GetCollisionObjectType (Variables|/Script/Engine.Character|GetCapsuleComponent _output_get)))
  (Collision|BindEventtoOnComponentEndOverlap (Variables|/Script/Engine.Character|GetCapsuleComponent _output_get) (delegate Custom|CharacterToSpawnEndOverlap))
  (Collision|SetCollisionObjectType (Variables|/Script/Engine.Character|GetCapsuleComponent _output_get) "ECC_GameTraceChannel1")
  (Input|DisableInput (Variables|Default|GetCharacterToSpawn) 0)
  (Variables|Default|SetIsSpawning true))

(event Custom|CharacterToSpawnEndOverlap
  (params (OverlappedComponent :type Primitive%20Component%20Object%20Reference) (OtherActor :type Actor%20Object%20Reference) (OtherComp :type Primitive%20Component%20Object%20Reference) (OtherBodyIndex :type Integer))
  (CallFunction|EndSpawn))

(event EventBeginPlay)

(event EventTick
  (params (DeltaSeconds :type Float%20%28single-precision%29))
  (if (Variables|Default|GetIsSpawning)
    (Variables|/Script/Engine.MovementComponent|SetVelocity (Variables|/Script/Engine.Character|GetCharacterMovement (Variables|Default|GetCharacterToSpawn)) (Math|Vector|MakeVector 0.0 0.0 (Variables|Default|GetSpawnVerticalSpeed)))))