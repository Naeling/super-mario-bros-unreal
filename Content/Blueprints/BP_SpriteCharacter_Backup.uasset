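; Paper2D Mario player character with walking, running, variable-height jumping, death and grow-to-big behavior.
; Tick drives walk and jump states, comparing facing with velocity or input to tune friction and air control and pick skid or walk flipbooks.
; Held jumps reapply timer-scaled upward velocity until release, timeout or head bump.
; Death and growth use timers for a collisionless death hop or a swap to big flipbooks and capsule.
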(event Custom|Update%20Walk%20Animation
  (if (== (Math|Vector|VectorLength (Variables|/Script/Engine.MovementComponent|GetVelocity (Variables|Character|GetCharacterMovement))) 0.0)
    (Sprite|SetFlipbook (Variables|Default|GetSprite) (Variables|Default|GetMarioIdleFlipbook))
    (else
      (bind _isorientationopposedtovelocity (CallFunction|IsOrientationOpposedtoVelocity))
      (if _isorientationopposedtovelocity
        (Sprite|SetFlipbook (Variables|Default|GetSprite) (Variables|Default|GetMarioStopFlipbook))
        (else
          (Sprite|SetFlipbook (Variables|Default|GetSprite) (Variables|Default|GetMarioWalkFlipbook))
          (CallFunction|UpdateWalkAnimationPlayRate))))))

(event Custom|EnemyKillMario
  (if (not (Variables|Default|GetIsMarioDead))
    (Variables|Default|SetIsMarioDead true)
    (Sprite|SetFlipbook (Variables|Default|GetSprite) "/Game/Sprites/Mario/Normal/Small/Die/FB_Small_Mario_Die.FB_Small_Mario_Die")
    (Variables|/Script/Engine.MovementComponent|SetVelocity (Variables|Character|GetCharacterMovement) "0, 0, 0")
    (Utilities|Time|SetTimerbyEvent (delegate Custom|MarioKillEndTimer) (Variables|Default|GetMarioKillTimer))))

(event Custom|ManageWalkState
  (if (Pawn|Components|CharacterMovement|IsWalking (Variables|Character|GetCharacterMovement))
    (CallFunction|UpdateWalkAnimation)
    (CallFunction|UpdateGroundedCharacterRotation)
    (CallFunction|UpdateGroundFriction)))

(event Custom|UpdateAirControl
  (bind _charactermovement (Variables|Character|GetCharacterMovement))
  (bind _charactermovement_2 (Variables|Character|GetCharacterMovement))
  (bind _isorientationopposedtomoverightinput (CallFunction|IsOrientationOpposedtoMoveRightInput))
  (bind _isorientationopposedtovelocity (CallFunction|IsOrientationOpposedtoVelocity))
  (if (or _isorientationopposedtovelocity _isorientationopposedtomoverightinput)
    (Variables|/Script/Engine.CharacterMovementComponent|SetMaxAcceleration _charactermovement 3e+02)
    (Variables|/Script/Engine.CharacterMovementComponent|SetFallingLateralFriction _charactermovement 0.8)
    (else
      (Variables|/Script/Engine.CharacterMovementComponent|SetMaxAcceleration _charactermovement_2 1.5e+02)
      (Variables|/Script/Engine.CharacterMovementComponent|SetFallingLateralFriction _charactermovement_2 0.0))))

(event Custom|ApplyKillVelocity
  (Character|Jump)
  (Collision|SetCollisionEnabled (Variables|Collision|GetCapsuleComponent) "NoCollision")
  (Variables|/Script/Engine.MovementComponent|SetVelocity (Variables|Character|GetCharacterMovement) (Math|Vector|MakeVector 0.0 0.0 (Variables|Default|GetMarioKillVelocity))))

(event Custom|Update%20Ground%20Friction
  (bind _isorientationopposedtovelocity (CallFunction|IsOrientationOpposedtoVelocity))
  (if _isorientationopposedtovelocity
    (Variables|/Script/Engine.CharacterMovementComponent|SetGroundFriction (Variables|Character|GetCharacterMovement) 3.3)
    (else
      (Variables|/Script/Engine.CharacterMovementComponent|SetGroundFriction (Variables|Character|GetCharacterMovement) 1.5))))

(event Custom|EndMarioGrowTimer
  (CallFunction|SetBigFlipbooks)
  (Components|Capsule|SetCapsuleSize (Variables|Collision|GetCapsuleComponent) 6.0 14.0 true)
  (Variables|Default|SetIsMarioChangingSize false)
  (Input|EnableInput 0))

(event Custom|Grow
  (if (not (Variables|Default|GetIsMarioChangingSize))
    (Variables|Default|SetIsMarioChangingSize true)
    (Input|DisableInput 0)
    (Variables|/Script/Engine.MovementComponent|SetVelocity (Variables|Character|GetCharacterMovement) "0, 0, 0")
    (Components|Timeline|SetPlayRate (Variables|Default|GetSprite) 1.0)
    (Sprite|SetFlipbook (Variables|Default|GetSprite) "/Game/Sprites/Mario/Normal/Small/Grow/FB_Mario_Grow.FB_Mario_Grow")
    (Utilities|Time|SetTimerbyEvent (delegate Custom|EndMarioGrowTimer) 0.8)))

(event Custom|UpdateWalkAnimationPlayRate
  (bind _charactermovement (Variables|Character|GetCharacterMovement))
  (if (Pawn|Components|CharacterMovement|IsWalking _charactermovement)
    (Components|Timeline|SetPlayRate (Variables|Default|GetSprite) (Math|Float|Max(Float) (* (Math|Float|Absolute(Float) (.X (Math|Vector|BreakVector (Variables|/Script/Engine.MovementComponent|GetVelocity _charactermovement)))) 0.01) 0.6))))

(event Custom|ApplyJumpVelocity
  (Variables|/Script/Engine.MovementComponent|SetVelocity (Variables|Character|GetCharacterMovement) (Math|Vector|MakeVector (.X (Class|KismetMathLibrary|BreakVector3f (Variables|/Script/Engine.MovementComponent|GetVelocity (Variables|Character|GetCharacterMovement)))) (.Y (Class|KismetMathLibrary|BreakVector3f (Variables|/Script/Engine.MovementComponent|GetVelocity (Variables|Character|GetCharacterMovement)))) (* (Variables|Default|GetJumpVelocity) (Math|Float|SafeDivide (Variables|Default|GetJumpInputMaxDuration) (Math|Float|Max(Float) (Class|KismetSystemLibrary|GetTimerElapsedTimeHandle (Variables|Default|GetJumpTimer)) 0.2))))))

(event Custom|StartMarioJumping
  (Variables|Default|SetIsMarioJumping true)
  (bind _returnvalue (Utilities|Time|SetTimerbyEvent (delegate Custom|EndTimerMarioJumpingEvent) (Variables|Default|GetJumpInputMaxDuration)))
  (Variables|Default|SetJumpTimer _returnvalue)
  (Character|Jump)
  (Sprite|SetFlipbook (Variables|Default|GetSprite) (Variables|Default|GetMarioJumpFlipbook)))

(event Custom|UpdateGroundedCharacterRotation
  (Utilities|IsValid (Pawn|GetController)
    (:Is%20Valid
      (Math|Float|CompareFloat (Input|AxisValues|GetMoveRight) 0.0
        (:>
          (Pawn|SetControlRotation (Pawn|GetController) (Math|Rotator|MakeRotator 0.0 0.0 0.0)))
        (:<
          (Pawn|SetControlRotation (Pawn|GetController) (Math|Rotator|MakeRotator 0.0 0.0 -1.8e+02)))))))

(event Custom|MarioKillEndTimer
  (CallFunction|ApplyKillVelocity))

(event Custom|StopMarioJumping
  (Variables|Default|SetIsMarioJumping false)
  (Character|StopJumping))

(event Custom|EndTimerMarioJumpingEvent
  (CallFunction|StopMarioJumping))

(event Custom|ManageJumpState
  (CallFunction|UpdateAirControl)
  (if (Variables|Default|GetIsMarioJumping)
    (CallFunction|ApplyJumpVelocity)))

(event EventBeginPlay)

(event Collision|EventHit
  (params (MyComp :type Primitive%20Component%20Object%20Reference) (Other :type Actor%20Object%20Reference) (OtherComp :type Primitive%20Component%20Object%20Reference) (bSelfMoved :type Boolean) (HitLocation :type Vector :default "0, 0, 0") (HitNormal :type Vector :default "0, 0, 0") (NormalImpulse :type Vector :default "0, 0, 0") (Hit :type Hit%20Result%20Structure%20%28by%20ref%29))
  (bind _charactermovement (Variables|Character|GetCharacterMovement))
  (if (== (.z HitNormal) -1.0)
    (Variables|/Script/Engine.MovementComponent|SetVelocity _charactermovement (Math|Vector|MakeVector (.x (Variables|/Script/Engine.MovementComponent|GetVelocity _charactermovement)) (.y (Variables|/Script/Engine.MovementComponent|GetVelocity _charactermovement)) 0.0))
    (CallFunction|StopMarioJumping)))

(event EventTick
  (params (DeltaSeconds :type Float%20%28single-precision%29))
  (if (not (or (Variables|Default|GetIsMarioDead) (Variables|Default|GetIsMarioChangingSize)))
    (CallFunction|ManageWalkState)
    (CallFunction|ManageJumpState)))

(event Input|ActionEvents|InputActionRun
  (params (Key :type Key%20Structure))
  (bind _charactermovement (Variables|Character|GetCharacterMovement))
  (:Pressed
    (Variables|/Script/Engine.CharacterMovementComponent|SetMaxWalkSpeed _charactermovement 2e+02))
  (:Released
    (Variables|/Script/Engine.CharacterMovementComponent|SetMaxWalkSpeed _charactermovement 1e+02)))

(event Input|ActionEvents|InputActionJump
  (params (Key :type Key%20Structure))
  (:Pressed
    (if (not (Variables|Default|GetIsMarioDead))
      (if (Pawn|Components|CharacterMovement|IsWalking (Variables|Character|GetCharacterMovement))
        (CallFunction|StartMarioJumping))))
  (:Released
    (CallFunction|StopMarioJumping)))

(event Input|AxisEvents|InputAxisMoveRight
  (params (AxisValue :type Float%20%28single-precision%29))
  (if (not (Variables|Default|GetIsMarioDead))
    (bind _isorientationopposedtovelocity (CallFunction|IsOrientationOpposedtoVelocity))
    (if (or (not (Pawn|Components|CharacterMovement|IsWalking (Variables|Character|GetCharacterMovement))) (and (not _isorientationopposedtovelocity) (Pawn|Components|CharacterMovement|IsWalking (Variables|Character|GetCharacterMovement))))
      (Pawn|Input|AddMovementInput "1.000000,0.000000,0.000000" AxisValue false))))

(fn ConstructionScript)

(fn IsOrientationOpposedtoVelocity
  (bind _isorientationopposedtovalue (CallFunction|IsOrientationOpposedtoValue (.X (Math|Vector|BreakVector (Variables|/Script/Engine.MovementComponent|GetVelocity (Variables|Character|GetCharacterMovement))))))
  (return _isorientationopposedtovalue))

(fn IsOrientationOpposedtoMoveRightInput
  (bind _isorientationopposedtovalue (CallFunction|IsOrientationOpposedtoValue (Input|AxisValues|GetMoveRight)))
  (return _isorientationopposedtovalue))

(fn IsOrientationOpposedtoValue
  (params (Value :type Float%20%28double-precision%29))
  (return (or (and (== (.Yaw (Math|Rotator|BreakRotator (Pawn|GetControlRotation :!class /Script/Engine.Pawn))) -1.8e+02) (> Value 0.0)) (and (< Value 0.0) (== (.Yaw (Math|Rotator|BreakRotator (Pawn|GetControlRotation :!class /Script/Engine.Pawn))) 0.0)))))

(fn SetBigFlipbooks
  (Variables|Default|SetMarioIdleFlipbook "/Game/Sprites/Mario/Normal/Big/Idle/FB_Big_Mario_Idle.FB_Big_Mario_Idle")
  (Variables|Default|SetMarioWalkFlipbook "/Game/Sprites/Mario/Normal/Big/Walk-Run/FB_Big_Mario_Walk.FB_Big_Mario_Walk")
  (Variables|Default|SetMarioJumpFlipbook "/Game/Sprites/Mario/Normal/Big/Jump/FB_Big_Mario_Jump.FB_Big_Mario_Jump")
  (Variables|Default|SetMarioStopFlipbook "/Game/Sprites/Mario/Normal/Big/Walk-Run/FB_Big_Mario_Stop.FB_Big_Mario_Stop"))