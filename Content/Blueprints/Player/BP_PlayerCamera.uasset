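; BP_PlayerCamera is a player camera component that holds its pivot at a set height while following its parent horizontally.
; On BeginPlay it caches its immediate parent component.
; Every Tick it sets its relative location to zero X and Y, with Z offset by PivotZValue minus the parent's world Z, cancelling the parent's vertical movement.
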(event Custom|UpdateRelativeLocation
  (Transformation|SetRelativeLocation (Math|Vector|MakeVector 0.0 0.0 (- (Variables|Default|GetPivotZValue) (.Z (Math|Vector|BreakVector (Transformation|GetWorldLocation (Variables|Default|GetParent)))))) false false))

(event Custom|Initialization
  (Variables|Default|SetParent (Utilities|Array|Get(acopy) (Class|SceneComponent|GetParentComponents))))

(event EventBeginPlay
  (CallFunction|Initialization))

(event EventTick
  (params (DeltaSeconds :type Float%20%28single-precision%29))
  (CallFunction|UpdateRelativeLocation))