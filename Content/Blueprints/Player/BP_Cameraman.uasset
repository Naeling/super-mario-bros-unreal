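; BP_Cameraman is a side-scroller camera carrier that follows Mario along X, snapping to a fixed offset ahead of him on BeginPlay.
; Each tick it sets its CharacterMovement velocity to Mario's positive X velocity times a multiplier, so it never moves backward, or to zero when static.
; Two detection volumes, low and high velocity, switch that multiplier as Mario overlaps or leaves them, stopping the follow when he exits the low zone.
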(event OnComponentBeginOverlap(ForwardMoveDetectionLowVelocity)
  (params (OverlappedComponent :type Primitive%20Component%20Object%20Reference) (OtherActor :type Actor%20Object%20Reference) (OtherComp :type Primitive%20Component%20Object%20Reference) (OtherBodyIndex :type Integer) (bFromSweep :type Boolean) (SweepResult :type Hit%20Result%20Structure%20%28by%20ref%29))
  (if (== OtherActor (Variables|Default|GetMarioActor))
    (Variables|Default|SetForwardVelocityMultiplier (Variables|Default|GetLowForwardVelocityMultiplier_0))))

(event OnComponentEndOverlap(ForwardMoveDetectionLowVelocity)
  (params (OverlappedComponent :type Primitive%20Component%20Object%20Reference) (OtherActor :type Actor%20Object%20Reference) (OtherComp :type Primitive%20Component%20Object%20Reference) (OtherBodyIndex :type Integer))
  (if (== OtherActor (Variables|Default|GetMarioActor))
    (Variables|Default|SetForwardVelocityMultiplier 0.0)))

(event OnComponentBeginOverlap(ForwardMoveDetectionHighVelocity)
  (params (OverlappedComponent :type Primitive%20Component%20Object%20Reference) (OtherActor :type Actor%20Object%20Reference) (OtherComp :type Primitive%20Component%20Object%20Reference) (OtherBodyIndex :type Integer) (bFromSweep :type Boolean) (SweepResult :type Hit%20Result%20Structure%20%28by%20ref%29))
  (if (== OtherActor (Variables|Default|GetMarioActor))
    (Variables|Default|SetForwardVelocityMultiplier (Variables|Default|GetHighForwardVelocityMultiplier))))

(event OnComponentEndOverlap(ForwardMoveDetectionHighVelocity)
  (params (OverlappedComponent :type Primitive%20Component%20Object%20Reference) (OtherActor :type Actor%20Object%20Reference) (OtherComp :type Primitive%20Component%20Object%20Reference) (OtherBodyIndex :type Integer))
  (if (== OtherActor (Variables|Default|GetMarioActor))
    (Variables|Default|SetForwardVelocityMultiplier (Variables|Default|GetLowForwardVelocityMultiplier_0))))

(event Custom|MoveToMarioPosition
  (bind _returnvalue (Transformation|GetActorLocation))
  (Transformation|SetActorLocation (Math|Vector|MakeVector (+ (.x (Transformation|GetActorLocation (Variables|Default|GetMarioActor))) 8e+01) (.y _returnvalue) (.z _returnvalue)) false false))

(event EventBeginPlay
  (bind _returnvalue (Actor|GetActorOfClass (Variables|Default|GetMarioClass)))
  (Variables|Default|SetMarioActor _returnvalue)
  (CallFunction|MovetoMarioPosition))

(event EventTick
  (params (DeltaSeconds :type Float%20%28single-precision%29))
  (bind _forwardvelocity (CallFunction|ComputeForwardVelocity))
  (Variables|/Script/Engine.MovementComponent|SetVelocity (Variables|Character|GetCharacterMovement) (Math|Vector|MakeVector _forwardvelocity 0.0 0.0)))

(fn ConstructionScript)

(fn IsMarioMovingForward
  (return (> (.x (Transformation|GetVelocity (Variables|Default|GetMarioActor))) 0.0)))

(fn ComputeForwardVelocity
  (if (Variables|Default|GetIsStatic)
    (return 0.0)
    (else
      (return (* (Math|Float|Max(Float) (.x (Transformation|GetVelocity (Variables|Default|GetMarioActor))) 0.0) (Variables|Default|GetForwardVelocityMultiplier))))))