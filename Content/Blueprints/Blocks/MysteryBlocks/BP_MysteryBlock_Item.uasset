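; Mystery block variant that releases an item when activated.
; It overrides OnBlockActivation, runs the parent behavior, then spawns the configured Item class at the block's location, regardless of collisions.
; The spawned actor is handed to CharacterSpawner's SpawnCharacter, while all other behavior comes from the parent block.
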(event EventBeginPlay
  (|CallParentFunction) ; This node is disabled and will not be called.\nDrag off pins to build functionality.
)

(event Collision|EventActorBeginOverlap
  (params (OtherActor :type Actor%20Object%20Reference))
  (|CallParentFunction OtherActor) ; This node is disabled and will not be called.\nDrag off pins to build functionality.
)

(event EventTick
  (params (DeltaSeconds :type Float%20%28single-precision%29))
  (|CallParentFunction DeltaSeconds) ; This node is disabled and will not be called.\nDrag off pins to build functionality.
)

(fn ConstructionScript
  (|CallParentFunction))

(fn OnBlockActivation
  (bind _returnvalue (Transformation|GetActorTransform))
  (|CallParentFunction)
  (bind _returnvalue_2 (Game|SpawnActorfromClass (Variables|Default|GetItem) (Math|Transform|MakeTransform (Math|Vector|MakeVector (.x (.location _returnvalue)) (.y (.location _returnvalue)) (.z (.location _returnvalue))) "0, 0, 0" "1.000000,1.000000,1.000000") "AlwaysSpawn" 0 0))
  (Default|SpawnCharacter (Variables|Default|GetCharacterSpawner) _returnvalue_2))