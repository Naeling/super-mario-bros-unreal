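; Mystery block variant that spawns a coin actor when activated.
; Overrides OnBlockActivation to run the parent's activation logic, then spawns CoinActor at the block's location, raised by ActorSpawnVerticalOffset.
; All other behavior comes from the parent class, as the event graph holds only disabled stubs and the construction script just calls the parent.
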(event EventBeginPlay
  (|CallParentFunction) ; This node is disabled and will not be called.\nDrag off pins to build functionality.
)

(event Collision|EventActorBeginOverlap
  (params (OtherActor :type Actor%20Object%20Reference))
  (|CallParentFunction OtherActor) ; This node is disabled and will not be called.\nDrag off pins to build functionality.
)

(event EventTick
  (params (DeltaSeconds :type Float%20%28single-precision%29))
  (|CallParentFunction DeltaSeconds) ; This node is disabled and will not be called.\nDrag off pins to build functionality.
)

(fn ConstructionScript
  (|CallParentFunction))

(fn OnBlockActivation
  (bind _returnvalue (Transformation|GetActorTransform))
  (|CallParentFunction)
  (Game|SpawnActorfromClass (Variables|Default|GetCoinActor) (Math|Transform|MakeTransform (Math|Vector|MakeVector (.x (.location _returnvalue)) (.y (.location _returnvalue)) (+ (.z (.location _returnvalue)) (Variables|Default|GetActorSpawnVerticalOffset))) "0, 0, 0" "1.000000,1.000000,1.000000") "Undefined" 0 0))