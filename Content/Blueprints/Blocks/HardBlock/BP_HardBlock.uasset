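; BP_HardBlock is a Mario-style breakable block that shatters when hit by a big Mario.
; It extends a parent block's OnBlockHit, then checks IsBig before spawning debris and destroying itself.
; SpawnAllChunks launches four quadrant sprites diagonally outward, with separate vertical speeds for top and bottom pairs.
; Each chunk spawns at the block's X and Z, with Y set to DisplayLayer for 2D layering.
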(event EventBeginPlay)

(event Collision|EventActorBeginOverlap
  (params (OtherActor :type Actor%20Object%20Reference)))

(event EventTick
  (params (DeltaSeconds :type Float%20%28single-precision%29)))

(fn ConstructionScript
  (|CallParentFunction))

(fn OnBlockHit
  (params (Mario%20Actor :type BP%20Sprite%20Character%20Object%20Reference))
  (|CallParentFunction Mario%20Actor)
  (if (Variables|/Game/Blueprints/Player/BP_SpriteCharacter.BP_SpriteCharacter_C|GetIsBig Mario%20Actor)
    (CallFunction|SpawnAllChunks)
    (Actor|DestroyActor)))

(fn SpawnChunk
  (params (Sprite :type Paper%20Sprite%20Object%20Reference) (LauchVelocity :type Vector))
  (bind _returnvalue (Transformation|GetActorLocation))
  (Game|SpawnActorfromClass (Variables|Default|GetChunkClass) (Math|Conversions|ToTransform(Vector) (Math|Vector|MakeVector (.x _returnvalue) (Variables|Default|GetDisplayLayer) (.z _returnvalue))) "Undefined" 0 LauchVelocity Sprite 0))

(fn SpawnAllChunks
  (CallFunction|SpawnChunk (Variables|Default|GetTopLeftChunkSprite) (Math|Vector|MakeVector (* (Variables|Default|GetHorizontalSpeed) -1.0) 0.0 (Variables|Default|GetTopVerticalSpeed)))
  (CallFunction|SpawnChunk (Variables|Default|GetTopRightChunkSprite) (Math|Vector|MakeVector (Variables|Default|GetHorizontalSpeed) 0.0 (Variables|Default|GetTopVerticalSpeed)))
  (CallFunction|SpawnChunk (Variables|Default|GetBottomLeftChunkSprite) (Math|Vector|MakeVector (* (Variables|Default|GetHorizontalSpeed) -1.0) 0.0 (Variables|Default|GetBottomVerticalSpeed)))
  (CallFunction|SpawnChunk (Variables|Default|GetBottomRightChunkSprite) (Math|Vector|MakeVector (Variables|Default|GetHorizontalSpeed) 0.0 (Variables|Default|GetBottomVerticalSpeed))))