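; Base Mario-style block that reacts when BP_SpriteCharacter, identified by class display name, hits it with a vertical hit normal of 1.
; OnBlockHit plays a timeline meant to bump the flipbook, enables KillEnemiesBox and starts the death animation on enemies already overlapping it.
; Enemies entering the box later die only while IsMovingUp is true.
; The timeline's finish handler disables the box's collision.
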(event OnComponentBeginOverlap(KillEnemiesBox)
  (params (OverlappedComponent :type Primitive%20Component%20Object%20Reference) (OtherActor :type Actor%20Object%20Reference) (OtherComp :type Primitive%20Component%20Object%20Reference) (OtherBodyIndex :type Integer) (bFromSweep :type Boolean) (SweepResult :type Hit%20Result%20Structure%20%28by%20ref%29))
  (bind _asbp_enemy (Utilities|Casting|CastToBP_Enemy OtherActor))
  (if (Variables|Default|GetIsMovingUp)
    (Default|StartDeathAnimation _asbp_enemy 1.0)))

(event Collision|EventHit
  (params (MyComp :type Primitive%20Component%20Object%20Reference) (Other :type Actor%20Object%20Reference) (OtherComp :type Primitive%20Component%20Object%20Reference) (bSelfMoved :type Boolean) (HitLocation :type Vector :default "0, 0, 0") (HitNormal :type Vector :default "0, 0, 0") (NormalImpulse :type Vector :default "0, 0, 0") (Hit :type Hit%20Result%20Structure%20%28by%20ref%29))
  (bind _ismarioactor (CallFunction|IsMarioActor Other))
  (if _ismarioactor
    (if (== (.Z (Math|Vector|BreakVector HitNormal)) 1.0)
      (bind _asbp_sprite_character (Utilities|Casting|CastToBP_SpriteCharacter Other))
      (CallFunction|OnBlockHit _asbp_sprite_character))))

(fn ConstructionScript)

(fn IsMarioActor
  (params (Actor :type Actor%20Object%20Reference))
  (return (Utilities|Enum|Equal(Enum) (Utilities|GetClassDisplayName (Utilities|GetClass Actor)) "BP_SpriteCharacter_C")))

(fn OnBlockHit
  (params (Mario%20Actor :type BP%20Sprite%20Character%20Object%20Reference))
  (Components|Timeline|PlayfromStart (Variables|Default|GetTimeline_0))
  (Collision|SetCollisionEnabled (Variables|Default|GetKillEnemiesBox) "QueryOnly")
  (for _array_element (Collision|GetOverlappingActors (Variables|Default|GetKillEnemiesBox) "/Game/Blueprints/Enemies/BP_Enemy.BP_Enemy_C" :!class /Script/Engine.PrimitiveComponent)
    (bind _asbp_enemy (Utilities|Casting|CastToBP_Enemy _array_element))
    (Default|StartDeathAnimation _asbp_enemy 1.0)))