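; BP_HardBlock is a Mario-style block that bounces when the player character hits it vertically.
; On Hit, it identifies Mario by comparing the class display name to BP_SpriteCharacter_C and requires a hit normal Z of exactly 1.
; The Bounce timeline then drives the Block component's relative Z.
; A bounds-based IsMarioBelowSelf helper is defined but not called here.
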(event EventBeginPlay)

(event Collision|EventActorBeginOverlap
  (params (OtherActor :type Actor%20Object%20Reference)))

(event EventTick
  (params (DeltaSeconds :type Float%20%28single-precision%29)))

(event Collision|EventHit
  (params (MyComp :type Primitive%20Component%20Object%20Reference) (Other :type Actor%20Object%20Reference) (OtherComp :type Primitive%20Component%20Object%20Reference) (bSelfMoved :type Boolean) (HitLocation :type Vector :default "0, 0, 0") (HitNormal :type Vector :default "0, 0, 0") (NormalImpulse :type Vector :default "0, 0, 0") (Hit :type Hit%20Result%20Structure%20%28by%20ref%29))
  (bind _block (Variables|Default|GetBlock))
  (bind _relativelocation (Variables|/Script/Engine.SceneComponent|GetRelativeLocation _block))
  (bind _ismarioactor (CallFunction|IsMarioActor Other))
  (if _ismarioactor
    (if (== (.Z (Math|Vector|BreakVector HitNormal)) 1.0)
      (bind _updown (Timeline|Bounce PlayFromStart)
        (:Update
          (Transformation|SetRelativeLocation (Variables|Default|GetBlock) (Math|Vector|MakeVector (.x _relativelocation) (.y _relativelocation) _updown) false false))))))

(fn ConstructionScript)

(fn IsMarioActor
  (params (Actor :type Actor%20Object%20Reference))
  (return (Utilities|Enum|Equal(Enum) (Utilities|GetClassDisplayName (Utilities|GetClass Actor)) "BP_SpriteCharacter_C")))

(fn IsMarioBelowSelf
  (params (Actor :type Actor%20Object%20Reference))
  (bind _returnvalue (Actor|GetComponentbyClass Actor "/Script/Engine.CapsuleComponent"))
  (bind (_origin _boxextent) (Collision|GetComponentBounds _returnvalue))
  (return (< (.Z (Math|Vector|BreakVector _origin)) (- (.Z (Math|Vector|BreakVector (Transformation|GetActorLocation))) (/ (.Z (Math|Vector|BreakVector _boxextent)) 4.0)))))