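; BP_MysteryBlock_Mushroom is a legacy one-shot mystery block that releases an item when Mario hits it.
; A Hit with a normal Z of exactly 1, from an actor matched by class-name string, deactivates the block and swaps its flipbook.
; It then spawns the Item class at a vertical offset, calls Spawn on it as BP_Item, and bounces the sprite via timeline.
; IsMarioBelowSelf is defined but unused.
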(event Collision|EventActorBeginOverlap
  (params (OtherActor :type Actor%20Object%20Reference)))

(event EventTick
  (params (DeltaSeconds :type Float%20%28single-precision%29)))

(event Collision|EventHit
  (params (MyComp :type Primitive%20Component%20Object%20Reference) (Other :type Actor%20Object%20Reference) (OtherComp :type Primitive%20Component%20Object%20Reference) (bSelfMoved :type Boolean) (HitLocation :type Vector :default "0, 0, 0") (HitNormal :type Vector :default "0, 0, 0") (NormalImpulse :type Vector :default "0, 0, 0") (Hit :type Hit%20Result%20Structure%20%28by%20ref%29))
  (bind _returnvalue (Transformation|GetActorTransform))
  (bind _flipbook (Variables|Default|GetFlipbook))
  (bind _relativelocation (Variables|/Script/Engine.SceneComponent|GetRelativeLocation _flipbook))
  (if (Variables|Default|GetIsActive)
    (bind _ismarioactor (CallFunction|IsMarioActor Other))
    (if _ismarioactor
      (if (== (.Z (Math|Vector|BreakVector HitNormal)) 1.0)
        (Variables|Default|SetIsActive false)
        (Sprite|SetFlipbook (Variables|Default|GetFlipbook) "/Game/Sprites/Worlds/Props/Blocks/MysteryBlock/Overworld/FB_MysteryBlock_Overworld_Inactive.FB_MysteryBlock_Overworld_Inactive")
        (bind _returnvalue_2 (Game|SpawnActorfromClass (Variables|Default|GetItem) (Math|Transform|MakeTransform (Math|Vector|MakeVector (.x (.location _returnvalue)) (.y (.location _returnvalue)) (+ (.z (.location _returnvalue)) (Variables|Default|GetActorSpawnVerticalOffset))) "0, 0, 0" "1.000000,1.000000,1.000000") "AlwaysSpawn" 0 0))
        (bind _asbp_mushroom (Utilities|Casting|CastToBP_Item _returnvalue_2))
        (Default|Spawn _asbp_mushroom)
        (bind _updown (Timeline|Bounce Play)
          (:Update
            (Transformation|SetRelativeLocation (Variables|Default|GetFlipbook) (Math|Vector|MakeVector (.x _relativelocation) (.y _relativelocation) _updown) false false)))))))

(fn ConstructionScript)

(fn IsMarioActor
  (params (Actor :type Actor%20Object%20Reference))
  (return (Utilities|Enum|Equal(Enum) (Utilities|GetClassDisplayName (Utilities|GetClass Actor)) "BP_SpriteCharacter_C")))

(fn IsMarioBelowSelf
  (params (Actor :type Actor%20Object%20Reference))
  (bind _returnvalue (Actor|GetComponentbyClass Actor "/Script/Engine.CapsuleComponent"))
  (bind (_origin _boxextent) (Collision|GetComponentBounds _returnvalue))
  (return (< (.Z (Math|Vector|BreakVector _origin)) (- (.Z (Math|Vector|BreakVector (Transformation|GetActorLocation))) (/ (.Z (Math|Vector|BreakVector _boxextent)) 4.0)))))