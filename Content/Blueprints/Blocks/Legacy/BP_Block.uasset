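; Legacy block Blueprint for a Mario-style game that reacts when the player sprite character hits it.
; A hit counts only when the actor's class name matches BP_SpriteCharacter_C and the hit normal points straight up.
; OnBlockHit then restarts a timeline by reference, whose UpDown track is set up to move the block's flipbook along relative Z as a bump animation.
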(event Collision|EventHit
  (params (MyComp :type Primitive%20Component%20Object%20Reference) (Other :type Actor%20Object%20Reference) (OtherComp :type Primitive%20Component%20Object%20Reference) (bSelfMoved :type Boolean) (HitLocation :type Vector :default "0, 0, 0") (HitNormal :type Vector :default "0, 0, 0") (NormalImpulse :type Vector :default "0, 0, 0") (Hit :type Hit%20Result%20Structure%20%28by%20ref%29))
  (bind _ismarioactor (CallFunction|IsMarioActor Other))
  (if _ismarioactor
    (if (== (.Z (Math|Vector|BreakVector HitNormal)) 1.0)
      (CallFunction|OnBlockHit))))

(fn ConstructionScript)

(fn IsMarioActor
  (params (Actor :type Actor%20Object%20Reference))
  (return (Utilities|Enum|Equal(Enum) (Utilities|GetClassDisplayName (Utilities|GetClass Actor)) "BP_SpriteCharacter_C")))

(fn OnBlockHit
  (Components|Timeline|PlayfromStart (Variables|Default|GetTimeline_0)))